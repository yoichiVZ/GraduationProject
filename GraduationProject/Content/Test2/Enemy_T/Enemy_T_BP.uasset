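; Enemy turret actor that fires Enemy_T_Bullet at intervals while active, with a Tick rotation meant to track the player.
; Overlap with a PlayerStart (not a pawn) sets IsActive and starts a looping Shoot timer at ShootingLate; end overlap clears IsActive, which gates Shoot.
; While active, Tick feeds its own location as both look-at start and target, and re-sets a debug "Hello" timer every frame.
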(event `self.ReceiveTick`
  (params (DeltaSeconds :type "Float (single-precision)"))
  ;[0 0.1331 1] Playerを見続ける処理
  (if (`self.isActive`)
    (`SceneComponent.K2_SetWorldRotation` (`self.DefaultSceneRoot`) (`KismetMathLibrary.FindLookAtRotation` (`self.K2_GetActorLocation`) (`self.K2_GetActorLocation`)) false false)
    ;[0 0.03511 1] 一定時間でShootイベントを呼び出す処理
    (bind _returnvalue (`KismetSystemLibrary.K2_SetTimer` null "test" (`self.ShootingLate`) true))))

(event `Shoot`
  ;[1 0 0] Shootイベント
  (if (`self.isActive`)
    (`|SpawnActorFromClass` "/Game/Test2/Enemy_T/Enemy_T_Bullet.Enemy_T_Bullet_C" (`self.GetTransform`) "Undefined" "OverrideRootScale" null null)))

(event `test`
  (`KismetSystemLibrary.PrintString` "Hello"))

(event `self.ReceiveActorBeginOverlap`
  (params (OtherActor :type "Actor Object Reference"))
  (cast `PlayerStart` OtherActor)
  (set `self.isActive` true)
  (bind _returnvalue (`KismetSystemLibrary.K2_SetTimer` null "Shoot" (`self.ShootingLate`) true)))

(event `self.ReceiveActorEndOverlap`
  (params (OtherActor :type "Actor Object Reference"))
  (cast `PlayerStart` OtherActor)
  (set `self.isActive` false)
  (setmembers `TimerHandle` :`StructRef` (stale `self.ReceiveActorBeginOverlap` _returnvalue)))

(fn `UserConstructionScript`)