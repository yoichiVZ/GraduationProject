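; Short-lived translucent afterimage of the player character, made of body, sword and shield meshes.
; The construction script gives each mesh a dynamic instance of its translucent material.
; Tick lowers their shared opacity linearly from a faint start according to the time elapsed since BeginPlay.
; BeginPlay records that start time and destroys the actor after DestroyTime, independently of the fade.
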(event `self.ReceiveBeginPlay`
  (set `self.Timer` (`KismetSystemLibrary.GetGameTimeInSeconds`))
  (`KismetSystemLibrary.Delay` (`self.DestroyTime`))
  (`self.K2_DestroyActor`))

(event `self.ReceiveTick`
  (params (DeltaSeconds :type "Float (single-precision)"))
  (bind _returnvalue (- 0.3 (- (`KismetSystemLibrary.GetGameTimeInSeconds`) (`self.Timer`))))
  (`MaterialInstanceDynamic.SetScalarParameterValue` (`self.MaterialInstance_Body`) "Opacity" _returnvalue)
  (`MaterialInstanceDynamic.SetScalarParameterValue` (`self.MaterialInstance_Sword`) "Opacity" _returnvalue)
  (`MaterialInstanceDynamic.SetScalarParameterValue` (`self.MaterialInstance_Shield`) "Opacity" _returnvalue))

(fn `UserConstructionScript`
  (bind _returnvalue (`PrimitiveComponent.CreateDynamicMaterialInstance` (`self.SkeletalMesh`) 0 "/Game/Resources/InfinityBladeWarriors/Character/CompleteCharacters/Textures_Materials/CharM_Golden/M_Char_Golden_Translucent.M_Char_Golden_Translucent" "None"))
  (set `self.MaterialInstance_Body` _returnvalue)
  (bind _returnvalue_2 (`PrimitiveComponent.CreateDynamicMaterialInstance` (`self.Sword`) 0 "/Game/Resources/Models/Weapons/Sword/Sword_Material_Translucent.Sword_Material_Translucent" "None"))
  (set `self.MaterialInstance_Sword` _returnvalue_2)
  (bind _returnvalue_3 (`PrimitiveComponent.CreateDynamicMaterialInstance` (`self.Shield`) 0 "/Game/Resources/Models/Weapons/Shield/ElvenShieldDeluxeBySARL_Material_Translucent.ElvenShieldDeluxeBySARL_Material_Translucent" "None"))
  (set `self.MaterialInstance_Shield` _returnvalue_3))