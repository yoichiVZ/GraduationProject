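; BP_FollowCamera is a camera actor that follows the first player's pawn.
; Every Tick it snaps itself to the pawn's location and the pawn's control rotation, with no interpolation or sweep.
; Unconnected leftover nodes would teleport it to a PlayerStart, make it the view target or place the Camera component behind the character, but none of them run.
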(event `self.ReceiveBeginPlay`)

(event `self.ReceiveTick`
  (params (DeltaSeconds :type "Float (single-precision)"))
  (bind _returnvalue (`GameplayStatics.GetPlayerPawn` 0))
  (`self.K2_SetActorLocation` (`self.K2_GetActorLocation` _returnvalue))
  (`self.K2_SetActorRotation` (`Pawn.GetControlRotation` _returnvalue)))

(fn `UserConstructionScript`)