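; Golem enemy character with melee, tackle and stone-throw attacks (throw marked unfinished) and an HP bar widget.
; Tick runs attacks from Notify-set flags and Blackboard keys, turning toward the player and toggling attack collision.
; Damage taken during the attack window checks for player parry, which stuns and halts AI logic; other hits drain a delayed-regen stun gauge.
; HP accumulates damage upward, with death at max and destruction once the disappear flag is set.
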(event `self.ReceiveDestroyed`
  (set `/Game/Character/Enemies/Enemy2/WBP_Golem_Bar.pParentChar` null (`self.HP_BarUI`)))

(event `self.ReceiveBeginPlay`
  (`PrimitiveComponent.SetCollisionEnabled` (`self.Attack_Collision`) "NoCollision")
  (bind _returnvalue (`|CreateWidget` "/Game/Character/Enemies/Enemy2/WBP_Golem_Bar.WBP_Golem_Bar_C" (`GameplayStatics.GetPlayerController` 0)))
  (bind _output_get (set `self.HP_BarUI` _returnvalue))
  (set `/Game/Character/Enemies/Enemy2/WBP_Golem_Bar.pParentChar` self _output_get)
  (`UserWidget.AddToViewport` _returnvalue 0))

(event `self.ReceiveTick`
  (params (DeltaSeconds :type "Float (single-precision)"))
  (if (`self.isDeath`)
    (set `/Game/Character/Enemies/Enemy2/WBP_Golem_Bar.pParentChar` null (`self.HP_BarUI`))
    (if (`self.isDissappear`)
      (`self.K2_DestroyActor`))
    (else
      (`self.SettingUI`)
      (bind _isdead (`self.GetIsAlive`))
      (if _isdead
        (set `self.isDeath` true)
        (elif (`self.isStan`)
          (`KismetSystemLibrary.Delay` (`self.Stan_Time`))
          (`self.FinishStan`)
          (else
            (`self.Attack1`)
            (`self.Tackle`)
            (`self.ThrowAttack`)
            (`self.HealStan`)))))))

(event `Attack1`
  ;[1 0 0] 処理が組み終わったもの
  ;;[1 0.5029 0] 近距離攻撃
  (if (`self.isAttackLook`)
    (`self.LookAtPlayer`))
  (`self.switching_AttackCollisionEnable`))

(event `ThrowAttack`
  (bind (_returnvalue_location _returnvalue_rotation) (`KismetMathLibrary.BreakTransform` (`self.GetTransform`)))
  ;[0 0.017 1] 未完成の処理
  ;;[1 0.5029 0] 投石処理
  (`self.ThrowIdle`)
  (if (`self.isThrow`)
    (bind _returnvalue (`|SpawnActorFromClass` "/Game/Character/Enemies/Enemy2/BP_Stone.BP_Stone_C" (`KismetMathLibrary.MakeTransform` _returnvalue_location _returnvalue_rotation (1.25 1.0 0.6)) "Undefined" "OverrideRootScale" null null))
    (`/Game/Character/Enemies/Enemy2/BP_Stone.settingOwner` _returnvalue self)
    (set `self.isThrow` false)
    (`KismetSystemLibrary.PrintString` "投げた")))

(event `HealStan`
  ;[1 0 0] 処理が組み終わったもの
  ;;[0 1 0] スタン値の回復処理
  (if (`self.isHealStan`)
    (`KismetSystemLibrary.Delay` 1.0)
    (`self.StanValue_Status`)
    (elif (>= (`self.WaitingCurrentTime_SV`) (`KismetMathLibrary.FTrunc` (* 10 (`self.WaitingMaxTime_SV`))))
      (set `self.isHealStan` true)
      (else
        (`KismetSystemLibrary.Delay` 0.1)
        (`/Engine/EditorBlueprintResources/StandardMacros.IncrementInt` (`self.WaitingCurrentTime_SV`))))))

(event `ThrowIdle`
  ;[1 0.5029 0] 投石待機処理
  (if (`BlackboardComponent.GetValueAsBool` (`AIBlueprintHelperLibrary.GetBlackboard` self) "Nageru_IdleFlag")
    (`self.LookAtPlayer`)))

(event `switching_AttackCollisionEnable`
  (bind _attack_collision (`self.Attack_Collision`))
  ;[1 0 0] 処理が組み終わったもの
  ;;[1 0.5029 0] 攻撃用の当たり判定のＯＮ/ＯＦＦ
  (if (`self.isAttackTime`)
    (`PrimitiveComponent.SetCollisionEnabled` _attack_collision "QueryAndPhysics")
    (else
      (`PrimitiveComponent.SetCollisionEnabled` _attack_collision "NoCollision"))))

(event `LookAtPlayer`
  (bind (_returnvalue_roll _returnvalue_pitch _returnvalue_yaw) (`KismetMathLibrary.BreakRotator` (`KismetMathLibrary.RInterpTo` (`self.K2_GetActorRotation`) (`KismetMathLibrary.FindLookAtRotation` (`self.K2_GetActorLocation`) (`self.K2_GetActorLocation` (`GameplayStatics.GetPlayerCharacter` 0))) (`GameplayStatics.GetWorldDeltaSeconds`) 15.0)))
  ;[0 0.017 1] 未完成の処理
  ;;[1 0.5029 0] プレイヤーの位置を向く処理
  (`self.K2_SetActorRotation` (`KismetMathLibrary.MakeRotator` _returnvalue_roll 0.0 _returnvalue_yaw)))

(event `ForwardAttack`
  (`self.K2_SetActorLocation` (+ (* (`KismetMathLibrary.GetForwardVector` (`self.K2_GetActorRotation`)) (`self.TackleSpeed`)) (`self.K2_GetActorLocation`))))

(event `CheckPlayerParry`
  ;[1 0 0] 処理が組み終わったもの
  ;;[0 0.017 1] Plyaerがパリィ状態か否か
  (`KismetSystemLibrary.PrintString` "パリィチェック！")
  (bind _asbp_action_character (cast `/Game/Character/Player/BP_Action_Character` (`GameplayStatics.GetPlayerCharacter` 0))
    (:`then`
      (if (and (`/Game/Character/Player/BP_Action_Character.Get Parry` _asbp_action_character) (`self.isAttackTime`))
        (`KismetSystemLibrary.PrintString` "パリィ成功")
        (set `self.isStan` true)
        (set `self.isAttackTime` false)
        (`BrainComponent.StopLogic` (`AIController.BrainComponent` (`AIBlueprintHelperLibrary.GetAIController` self)) "")
        (`MovementComponent.StopMovementImmediately` (`self.CharacterMovement`))
        (else
          (`KismetSystemLibrary.PrintString` "パリィ失敗"))))
    (:`CastFailed`
      (`KismetSystemLibrary.PrintString` "パリィチェック失敗" true true (struct :`G` 1.0 :`A` 1.0)))))

(event `Test`
  (bind _returnvalue (`self.K2_GetActorLocation`))
  ;[0 0.017 1] 未完成の処理
  (bind _outlaunchvelocity (`GameplayStatics.SuggestProjectileVelocity_CustomArc` _returnvalue (+ (200.0 200.0 0.0) (`SceneComponent.K2_GetComponentLocation` (`self.Mesh`)))))
  (`KismetSystemLibrary.PrintString` (`KismetStringLibrary.Conv_VectorToString` _outlaunchvelocity))
  (`GameplayStatics.Blueprint_PredictProjectilePath_ByTraceChannel` :`StartPos` _returnvalue :`LaunchVelocity` _outlaunchvelocity :`DrawDebugType` "ForDuration"))

(event `Tackle`
  (bind _returnvalue (`AIBlueprintHelperLibrary.GetBlackboard` self))
  (if (`BlackboardComponent.GetValueAsBool` (`AIBlueprintHelperLibrary.GetBlackboard` self) "Tackle_IdleFlag")
    (`self.LookAtPlayer`)
    (elif (`BlackboardComponent.GetValueAsBool` (`AIBlueprintHelperLibrary.GetBlackboard` self) "TackleFlag")
      (`self.ForwardAttack`)
      (`KismetSystemLibrary.Delay` 1.5)
      (`BlackboardComponent.SetValueAsBool` _returnvalue "Tackle_HitFlag" true)
      (`BlackboardComponent.SetValueAsBool` _returnvalue "TackleFlag" false))))

(event `self.ReceiveAnyDamage`
  (params (Damage :type "Float (single-precision)") (DamageType :type "DamageType Object Reference") (InstigatedBy :type "Controller Object Reference") (DamageCauser :type "Actor Object Reference"))
  ;[1 0 0] 処理が組み終わったもの
  ;;[1 0.9141 0.7977] 攻撃を食らう処理
  (if (`self.isAttackTime`)
    (`self.CheckPlayerParry`)
    (else
      (if (`self.isStan`)
        (`KismetSystemLibrary.PrintString` "攻撃された（スタン中" true true (struct :`R` 1.0 :`G` 0.983068 :`A` 1.0))
        (else
          (set `self.Stan_CurrentValue` (- (`self.Stan_CurrentValue`) 0.4))))
      (set `self.HP_CurrentValue` (+ (`self.HP_CurrentValue`) Damage))
      (`self.CheckIsStan`)
      (set `self.isHealStan` false)
      (set `self.WaitingCurrentTime_SV` 0)
      (`NiagaraFunctionLibrary.SpawnSystemAtLocation` "/Game/Effect/Damage_Set/Damage.Damage" (`self.K2_GetActorLocation`) (struct) (1.0 1.0 1.0) true true "AutoRelease"))))

(event `self.Attack_Collision.OnComponentBeginOverlap`
  (params (OverlappedComponent :type "PrimitiveComponent Object Reference") (OtherActor :type "Actor Object Reference") (OtherComp :type "PrimitiveComponent Object Reference") (OtherBodyIndex :type Integer) (bFromSweep :type Boolean) (SweepResult :type "HitResult Structure (by ref)"))
  ;[1 0 0] 処理が組み終わったもの
  ;;[1 0.5 0] 攻撃を与える処理
  (if (not (`self.isStan`))
    (bind _asbp_action_character (cast `/Game/Character/Player/BP_Action_Character` OtherActor))
    (if (`KismetMathLibrary.Conv_IntToBool` (`KismetMathLibrary.And_IntInt` (`KismetMathLibrary.Conv_BoolToInt` (== (`Character.CapsuleComponent` _asbp_action_character) OtherComp)) (`KismetMathLibrary.Conv_BoolToInt` (`self.isAttackTime`))))
      (`GameplayStatics.ApplyDamage` OtherActor 1.0 null self)
      (set `self.isAttackTime` false))))

(event `FinishStan`
  ;[1 0 0] 処理が組み終わったもの
  ;;[1 1 1] スタン終了処理
  (set `self.isStan` false)
  (set `self.Stan_CurrentValue` 1.0)
  (`CharacterMovementComponent.SetMovementMode` (`self.CharacterMovement`) "MOVE_Walking" 0)
  (`BrainComponent.RestartLogic` (`AIController.BrainComponent` (`AIBlueprintHelperLibrary.GetAIController` self)))
  (`KismetSystemLibrary.PrintString` "スタン終わり"))

(event `SettingUI`
  (bind _hp_barui (`self.HP_BarUI`))
  ;[1 0 0] 処理が組み終わったもの
  ;;[1 1 1] UI
  (if (`KismetSystemLibrary.IsValid` _hp_barui)
    (`/Game/Character/Enemies/Enemy2/WBP_Golem_Bar.SetUpdateGaugePosition` _hp_barui self)))

(fn `CameraShake`
  (`/Engine/EditorBlueprintResources/StandardMacros.DoOnce` false
    (:`Completed`
      (`PlayerCameraManager.StartCameraShake` :`self` (`GameplayStatics.GetPlayerCameraManager` 0) :`ShakeClass` "/Game/Character/Player/Camera/CameraShakeSourse_Golem.CameraShakeSourse_Golem_C")
      (`KismetSystemLibrary.PrintString` "揺れた"))))

(fn `CheckIsStan`
  (set `self.isStan` (<= (`self.Stan_CurrentValue`) 0.0)))

(fn `GetIsAlive`
  (returns (IsDead :type Boolean))
  (return (>= (`self.HP_CurrentValue`) (`self.HP_MaxValue`))))

(fn `Notify Activate Attack Time`
  (set `self.isAttackTime` true))

(fn `Notify Activate AttackLook`
  (set `self.isAttackLook` true))

(fn `Notify Activate Dissappear`
  (set `self.isDissappear` true))

(fn `Notify Activate Throw`
  (set `self.isThrow` true))

(fn `Notify Activate ThrowIdle`
  (set `self.isThrowIdle` true))

(fn `Notify DisActivate Attack Time`
  (set `self.isAttackTime` false))

(fn `Notify DisActivate AttackLook`
  (set `self.isAttackLook` false))

(fn `Notify DisActivate ThrowIdle`
  (set `self.isThrowIdle` false))

(fn `StanValue_Status`
  (bind _stan_currentvalue (`self.Stan_CurrentValue`))
  (if (`self.isHealStan`)
    (if (and (> _stan_currentvalue 0.0) (<= _stan_currentvalue (`self.Stan_MaxValue`)))
      (bind _output_get (set `self.Stan_CurrentValue` (`KismetMathLibrary.FClamp` (+ (`self.Stan_CurrentValue`) (`self.Stan_HealValue`)) 0.0 (`self.HP_MaxValue`))))
      (`KismetSystemLibrary.PrintString` "スタン値回復中" true true (struct :`R` 1.0 :`G` 0.016488 :`B` 0.79493 :`A` 1.0) 0.5)
      (`KismetSystemLibrary.PrintString` (`KismetStringLibrary.Concat_StrStr` "現在のスタン値は" (`KismetStringLibrary.Conv_DoubleToString` _output_get)) true true (struct :`R` 1.0 :`G` 0.847055 :`A` 1.0) 0.5))))

(fn `UserConstructionScript`)