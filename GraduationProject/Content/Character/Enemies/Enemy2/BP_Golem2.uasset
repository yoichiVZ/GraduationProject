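; BP_Golem2 is an AI-driven melee enemy with parry and stun mechanics.
; Notify functions toggle an attack window for overlap damage; hits inside it check for player parries, which stun the golem.
; Other hits raise HP toward a death threshold, flash the body color and drain a stun gauge, halting AI logic when stunned.
; Tick and BeginPlay are empty, leaving collision switching, UI updates, death and stun recovery unwired.
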(event `self.ReceiveDestroyed`
  ;[0 1 0.3419] 本体の死亡時にＵＩ破壊
  (set `/Game/Character/Enemies/Enemy1/WBP_ZombieBar.pParentChar` null (`self.HP_BarUI`)))

(event `self.ReceiveBeginPlay`)

(event `self.ReceiveTick`
  (params (DeltaSeconds :type "Float (single-precision)")))

(event `swtching_AttackCollisionEnable`
  (bind _attack_collision (`self.Attack_Collision`))
  ;[0 0.9131 1] 当たり判定の切り替え
  (if (`self.isAttackTime`)
    (`PrimitiveComponent.SetCollisionEnabled` _attack_collision "QueryAndPhysics")
    (else
      (`PrimitiveComponent.SetCollisionEnabled` _attack_collision "NoCollision"))))

(event `SettingUI`
  (bind _hp_barui (`self.HP_BarUI`))
  ;[0 0.9131 1] ゲージの表示
  (if (`KismetSystemLibrary.IsValid` _hp_barui)
    (`/Game/Character/Enemies/Enemy1/WBP_ZombieBar.SetUpdateGaugePosition` _hp_barui self)))

(event `DamageEffect`
  ;[0 0.9131 1] ダメージ食らった時の簡易的なエフェクト処理
  (`KismetSystemLibrary.PrintText` "ダメージ！！(エネミー")
  (bind _returnvalue (`PrimitiveComponent.CreateDynamicMaterialInstance` (`self.Mesh`) 0 null "None"))
  (`MaterialInstanceDynamic.SetVectorParameterValue` _returnvalue "BodyColor" (`self.Damage_Color`))
  (`KismetSystemLibrary.Delay` 1.0)
  (bind _returnvalue_2 (`PrimitiveComponent.CreateDynamicMaterialInstance` (`self.Mesh`) 0 "/Game/Resources/Textures/ZombieTextures/DefaultMaterial_Base_Color2_Mat.DefaultMaterial_Base_Color2_Mat" "None"))
  (`MaterialInstanceDynamic.SetVectorParameterValue` _returnvalue_2 "None" (`self.Default_Color`)))

(event `Check_PlayerParry`
  ;[0 0.9131 1] プレイヤーがパリィしたかを取得
  (bind _asbp_action_character (cast `/Game/Character/Player/BP_Action_Character` (`GameplayStatics.GetPlayerCharacter` 0)))
  (if (`/Game/Character/Player/BP_Action_Character.Get Parry` _asbp_action_character)
    (if (`self.isAttackTime`)
      (`KismetSystemLibrary.PrintString` "パリィ成功")
      (set `self.isStan` true)
      (set `self.isAttackTime` false)
      (`BrainComponent.StopLogic` (`AIController.BrainComponent` (`AIBlueprintHelperLibrary.GetAIController` self)) "")
      (`MovementComponent.StopMovementImmediately` (`self.CharacterMovement`))
      (else
        (`KismetSystemLibrary.PrintString` "パリィ失敗")))))

(event `self.ReceiveAnyDamage`
  (params (Damage :type "Float (single-precision)") (DamageType :type "DamageType Object Reference") (InstigatedBy :type "Controller Object Reference") (DamageCauser :type "Actor Object Reference"))
  ;[1 0.007369 0.04916] プレイヤーからダメージを受けた時の処理
  ;;[0 0.8963 1] 攻撃中か否か
  (if (`self.isAttackTime`)
    (`self.Check_PlayerParry`) ; プレイヤーがパリィしたか否か
    (else
      ;;[0 0.8963 1] スタン中か否かの処理
      (if (`self.isStan`)
        (set `self.isStan` false) ; スタン状態であったなら解除する
        (else
          (set `self.StanValue` (- (`self.StanValue`) 0.4)) ; スタン状態でなかったらスタン値をためる
        ))
      (set `self.HP` (+ (`self.HP`) 0.2))
      (`self.DamageEffect`)
      (`self.CheckIsStan`)
      (if (`self.isStan`)
        (`BrainComponent.StopLogic` (`AIController.BrainComponent` (`AIBlueprintHelperLibrary.GetAIController` self)) "")
        (`MovementComponent.StopMovementImmediately` (`self.CharacterMovement`))))))

(event `self.Attack_Collision.OnComponentBeginOverlap`
  (params (OverlappedComponent :type "PrimitiveComponent Object Reference") (OtherActor :type "Actor Object Reference") (OtherComp :type "PrimitiveComponent Object Reference") (OtherBodyIndex :type Integer) (bFromSweep :type Boolean) (SweepResult :type "HitResult Structure (by ref)"))
  ;[0.9734 0 0] プレイヤーにダメージを与える
  (if (not (`self.isStan`))
    (bind _asbp_action_character (cast `/Game/Character/Player/BP_Action_Character` OtherActor))
    (if (`KismetMathLibrary.Conv_IntToBool` (`KismetMathLibrary.And_IntInt` (`KismetMathLibrary.Conv_BoolToInt` (== (`Character.CapsuleComponent` _asbp_action_character) OtherComp)) (`KismetMathLibrary.Conv_BoolToInt` (`self.isAttackTime`))))
      (`GameplayStatics.ApplyDamage` OtherActor 1.0)
      (set `self.isAttackTime` false))))

(event `LookAtPlayer`
  ;[0.9734 0 0] 攻撃中にプレイヤーの向きを向く
  (`self.K2_SetActorRotation` (`KismetMathLibrary.RInterpTo` (`self.K2_GetActorRotation`) (`KismetMathLibrary.FindLookAtRotation` (`self.K2_GetActorLocation`) (`self.K2_GetActorLocation` (`GameplayStatics.GetPlayerCharacter` 0))) (`GameplayStatics.GetWorldDeltaSeconds`) 5.0)))

(event `Back`
  (bind (_returnvalue_x _returnvalue_y) (`KismetMathLibrary.BreakVector` (`self.K2_GetActorLocation`)))
  (bind (_point_x _point_y) (`KismetMathLibrary.BreakVector` (`self.point`)))
  ;[1 1 1] プレイヤーが後ろから攻撃してきたら
  (bind _output_get (set `self.point` (+ (`self.K2_GetActorLocation`) (`SceneComponent.GetForwardVector` (`self.CapsuleComponent`)))))
  (`KismetSystemLibrary.PrintString` (`KismetStringLibrary.Conv_DoubleToString` (`KismetMathLibrary.DegAtan2` (- (`KismetMathLibrary.MultiplyMultiply_FloatFloat` 0.0 _returnvalue_y) (`KismetMathLibrary.MultiplyMultiply_FloatFloat` _point_y 2.0)) (- (`KismetMathLibrary.MultiplyMultiply_FloatFloat` _returnvalue_x 2.0) (`KismetMathLibrary.MultiplyMultiply_FloatFloat` _point_x 2.0))))))

(fn `Attack`
  (if (`self.isAttacking`)
    (`self.PlayAnimMontage` "/Game/Resources/Animations/Zombie/Zombie_Attack_Mon.Zombie_Attack_Mon")))

(fn `CheckIsStan`
  (set `self.isStan` (<= (`self.StanValue`) 0.0)))

(fn `GetAttackTime`
  (returns (isAttackTime :type Boolean))
  (return (`self.isAttackTime`)))

(fn `GetIsAlive`
  (returns (IsAlive :type Boolean))
  (return (>= (`self.HP`) 1.0)))

(fn `GetIsStan`
  (returns (IsStan :type Boolean))
  (return (`self.isStan`)))

(fn `GetRandomLocation`
  (returns (Location :type "Vector Structure"))
  (bind _movearea (`self.MoveArea`))
  (bind (_origin _boxextent) (`KismetSystemLibrary.GetComponentBounds` (`TriggerBase.CollisionComponent` _movearea)))
  (`/Engine/EditorBlueprintResources/StandardMacros.IsValid` _movearea
    (:`Is Valid`
      (return (`KismetMathLibrary.RandomPointInBoundingBox` _origin _boxextent)))
    (:`Is Not Valid`
      (return (0.0 0.0 0.0)))))

(fn `Notify Activate Attack Time`
  (set `self.isAttackTime` true))

(fn `Notify DisActivate Attack Time`
  (set `self.isAttackTime` false))

(fn `UserConstructionScript`)