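; BP_GroundAttack is an enemy ground attack hazard that damages the player's capsule on overlap, crediting the owner passed through SettingOwner.
; Tick starts a one-time LifeTime countdown and uses a SpawnTime delay to repeatedly spawn the ground effect and falling-rock sound at its location.
; It destroys itself after its lifetime expires or when its box overlaps anything other than the player character or BP_Enemy2.
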(event `self.ReceiveTick`
  (params (DeltaSeconds :type "Float (single-precision)"))
  (bind (_returnvalue_location _returnvalue_rotation) (`KismetMathLibrary.BreakTransform` (`self.GetTransform`)))
  (`|ExecutionSequence`
    (:`then_0`
      (`/Engine/EditorBlueprintResources/StandardMacros.DoOnce` false
        (:`Completed`
          (`KismetSystemLibrary.Delay` (`self.lifeTime`))
          (set `self.isDead` true))))
    (:`then_1`
      (`KismetSystemLibrary.Delay` (`self.spawnTime`))
      (if (`self.isDead`)
        (`self.K2_DestroyActor`)
        (else
          (`GameplayStatics.SpawnEmitterAtLocation` "/Game/Effect/Particle/EnemyEffects/Golem/GroundAttackEffect.GroundAttackEffect" _returnvalue_location (struct) (0.18 0.7 0.05))
          (`GameplayStatics.PlaySound2D` "/Game/Resources/Sound/SE/EnemiesSE/Golem/岩が落ちる.岩が落ちる" 1.0 1.0 0.0 null null))))))

(event `self.Box.OnComponentBeginOverlap`
  (params (OverlappedComponent :type "PrimitiveComponent Object Reference") (OtherActor :type "Actor Object Reference") (OtherComp :type "PrimitiveComponent Object Reference") (OtherBodyIndex :type Integer) (bFromSweep :type Boolean) (SweepResult :type "HitResult Structure (by ref)"))
  (bind _asbp_action_character (cast `/Game/Character/Player/BP_Action_Character` OtherActor)
    (:`then`
      (if (== (`Character.CapsuleComponent` _asbp_action_character) OtherComp)
        (`GameplayStatics.ApplyDamage` OtherActor 0.4 null (`self.owner_s`))
        (`KismetSystemLibrary.PrintString` "Hello")
        (`GameplayStatics.PlaySound2D` "/Game/Resources/Sound/SE/EnemiesSE/rockBreak.rockBreak" 1.0 1.0 0.0 null null)))
    (:`CastFailed`
      (cast `/Game/Character/Enemies/Enemy2/BP_Enemy2` OtherActor
        (:`CastFailed`
          (`self.K2_DestroyActor`))))))

(fn `setting_owner`
  (params (owner_s :type "/Game/Character/Enemies/Enemy2/BP_Enemy2 Object Reference"))
  (set `self.owner_s` owner_s))

(fn `UserConstructionScript`)