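; BP_Stone is a spinning stone hazard, apparently thrown by Enemy2, that damages the player character.
; Tick tumbles it in pitch and roll, while SettingOwner stores the damage causer.
; Its sphere overlap applies damage only through the player's capsule, prints the owner's name for debugging, then destroys the stone.
; It ignores BP_Enemy2 and other player components, and destroys itself on overlapping any other actor.
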(event `self.Sphere.OnComponentBeginOverlap`
  (params (OverlappedComponent :type "PrimitiveComponent Object Reference") (OtherActor :type "Actor Object Reference") (OtherComp :type "PrimitiveComponent Object Reference") (OtherBodyIndex :type Integer) (bFromSweep :type Boolean) (SweepResult :type "HitResult Structure (by ref)"))
  (bind _owner_s (`self.owner_s`))
  (bind _asbp_action_character (cast `/Game/Character/Player/BP_Action_Character` OtherActor)
    (:`then`
      (if (== (`Character.CapsuleComponent` _asbp_action_character) OtherComp)
        (`GameplayStatics.ApplyDamage` OtherActor 1.0 null _owner_s)
        (`KismetSystemLibrary.PrintString` (`KismetStringLibrary.Concat_StrStr` "オーナーは：" (`KismetSystemLibrary.GetDisplayName` _owner_s)))
        (`self.K2_DestroyActor` :!label _label)))
    (:`CastFailed`
      (cast `/Game/Character/Enemies/Enemy2/BP_Enemy2` OtherActor
        (:`CastFailed`
          (goto _label))))))

(event `self.ReceiveTick`
  (params (DeltaSeconds :type "Float (single-precision)"))
  (bind _returnvalue (* (`self.Pitch Per Second`) DeltaSeconds))
  (`self.K2_AddActorLocalRotation` (`KismetMathLibrary.MakeRotator` (* _returnvalue -0.5) _returnvalue)))

(fn `settingOwner`
  (params (NewParam :type "/Game/Character/Enemies/Enemy2/BP_Enemy2 Object Reference"))
  (set `self.owner_s` NewParam))

(fn `UserConstructionScript`)