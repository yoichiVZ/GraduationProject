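; Test actor for a golem stone enemy piece built on a destructible mesh.
; The Hit event spawns enlarged explosion and smoke emitters attached to the mesh, gated by a DoOnce.
; Its binding to the mesh's fracture event is never executed, so fracturing does not trigger Hit within this Blueprint.
; An overlap handler destroys the actor when the overlapping actor differs from the GolemStoneDM reference.
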(event `self.ReceiveBeginPlay`)

(event `Hit`
  (params (HitPoint :type "Vector Structure (by ref)") (HitDirection :type "Vector Structure (by ref)"))
  (`|ExecutionSequence`
    (:`then_0`
      (`/Engine/EditorBlueprintResources/StandardMacros.DoOnce` false
        (:`Completed`
          (`GameplayStatics.SpawnEmitterAttached` "/Game/Resources/StarterContent/Particles/P_Explosion.P_Explosion" (`self.Golem_Stone_DM`) "None" (0.0 0.0 0.0) (struct) (5.0 5.0 5.0))
          (`GameplayStatics.SpawnEmitterAttached` "/Game/Resources/StarterContent/Particles/P_Smoke.P_Smoke" (`self.Golem_Stone_DM`) "None" (0.0 0.0 0.0) (struct) (5.0 5.0 5.0)))))))

(event `self.Golem_Stone_DM.OnComponentBeginOverlap`
  (params (OverlappedComponent :type "PrimitiveComponent Object Reference") (OtherActor :type "Actor Object Reference") (OtherComp :type "PrimitiveComponent Object Reference") (OtherBodyIndex :type Integer) (bFromSweep :type Boolean) (SweepResult :type "HitResult Structure (by ref)"))
  (if (!= OtherActor (`self.Golem_Stone_DM`))
    (`self.K2_DestroyActor`)))

(fn `UserConstructionScript`)