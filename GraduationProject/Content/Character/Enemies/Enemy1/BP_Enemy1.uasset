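; Zombie enemy character that spawns with an effect, faces the player, tackles, attacks and shows an HP bar.
; Tick handles state, exchanging Blackboard flags with BT_Enemy1 for spawn, tackle, attack, hit reactions and death.
; AnyDamage accumulates damage toward MaxHP, drains a stun gauge, and detects back hits by comparing yaw with the player's.
; Notify functions toggle attack collision, and a dynamic material tints the body by manager-provided type.
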(event `self.ReceiveDestroyed`
  ;[0 1 0.3419] 本体の死亡時にＵＩ破壊
  (set `/Game/Character/Enemies/Enemy1/WBP_ZombieBar.pParentChar` null (`self.HP_BarUI`)))

(event `swtching_AttackCollisionEnable`
  (bind _attack_collision (`self.Attack_Collision`))
  ;[1 1 1] 使ってない
  ;;[0 0.9131 1] 当たり判定の切り替え
  (if (`self.isAttackTime`)
    (`PrimitiveComponent.SetCollisionEnabled` _attack_collision "QueryAndPhysics")
    (else
      (`PrimitiveComponent.SetCollisionEnabled` _attack_collision "NoCollision"))))

(event `self.ReceiveBeginPlay`
  (bind (_returnvalue_x _returnvalue_y) (`KismetMathLibrary.BreakVector` (`self.K2_GetActorLocation`)))
  (bind (_returnvalue_x_2 _returnvalue_y_2) (`KismetMathLibrary.BreakVector` (`self.K2_GetActorLocation` (`GameplayStatics.GetPlayerPawn` 0))))
  (`PrimitiveComponent.SetCollisionEnabled` (`self.Attack_Collision`) "NoCollision") ; 攻撃用の当たり判定をとれないようにする
  (`PrimitiveComponent.SetCollisionEnabled` (`self.Tackle_Collision`) "NoCollision") ; 攻撃用の当たり判定をとれないようにする
  (`self.K2_SetActorRotation` (`KismetMathLibrary.MakeRotator` 0.0 0.0 (`KismetMathLibrary.DegAtan2` (- _returnvalue_y_2 _returnvalue_y) (- _returnvalue_x_2 _returnvalue_x)))) ; 生成時にプレイヤーの方向を向くよう
  (`self.setEnemyColor`))

(event `DamageEffect`
  ;[1 1 1] 使ってない
  ;;[0 0.9131 1] ダメージ食らった時の簡易的なエフェクト処理
  (`KismetSystemLibrary.PrintText` "ダメージ！！(エネミー")
  (bind _returnvalue (`PrimitiveComponent.CreateDynamicMaterialInstance` (`self.Mesh`) 0 "/Game/Resources/Textures/ZombieTextures/DefaultMaterial_Base_Color2_Mat.DefaultMaterial_Base_Color2_Mat" "None"))
  (`MaterialInstanceDynamic.SetVectorParameterValue` _returnvalue "BodyColor" (`self.Damage_Color`))
  (`KismetSystemLibrary.Delay` 1.0)
  (bind _returnvalue_2 (`PrimitiveComponent.CreateDynamicMaterialInstance` (`self.Mesh`) 0 "/Game/Resources/Textures/ZombieTextures/DefaultMaterial_Base_Color2_Mat.DefaultMaterial_Base_Color2_Mat" "None"))
  (`MaterialInstanceDynamic.SetVectorParameterValue` _returnvalue_2 "BodyColor" (`self.Default_Color`)))

(event `self.ReceiveTick`
  (params (DeltaSeconds :type "Float (single-precision)"))
  (if (`BlackboardComponent.GetValueAsBool` (`AIBlueprintHelperLibrary.GetBlackboard` self) "SpawnEndFlag")
    (if (`self.isDeath`)
      (if (`self.isDisappear`)
        (`self.K2_DestroyActor`))
      (else
        (`self.テストＨＰ`)
        (`self.SettingUI`)
        (if (`self.isStan`)
          ;[0.9625 1 0.2906] スタン中が終わった時の処理
          (`KismetSystemLibrary.Delay` (`self.StanTime`))
          (`self.FinishStan`)
          (elif (`self.isDamaging`)
            (`self.Damage`)
            (else
              (if (`self.isBack`)
                (`self.BackDamage`)
                (`KismetSystemLibrary.Delay` 0.3) ; 背面から攻撃を食らってから振りむこうとするまでの時間
                (`self.LookAtPlayer`)
                (`KismetSystemLibrary.Delay` 2.5)
                (set `self.isBack` false)
                (`BlackboardComponent.SetValueAsBool` (`AIBlueprintHelperLibrary.GetBlackboard` self) "AttackFlag" false)
                (else
                  (`self.Tackle`)))
              (`self.CheckIsStan`))))))
    (else
      (`/Engine/EditorBlueprintResources/StandardMacros.DoOnce` false
        (:`Completed`
          (`GameplayStatics.SpawnEmitterAtLocation` "/Game/Effect/Particle/EnemyEffects/Zombi/SpawnEffect/p_spawn_Numa.p_spawn_Numa" (`SceneComponent.K2_GetComponentLocation` (`self.Mesh`)))
          (`KismetSystemLibrary.Delay` 2.4)
          (`BlackboardComponent.SetValueAsBool` (`AIBlueprintHelperLibrary.GetBlackboard` self) "SpawnEndFlag" true))))))

(event `Check_PlayerParry`
  ;[1 1 1] 使ってない
  ;;[0 0.9131 1] プレイヤーがパリィしたかを取得
  (bind _asbp_action_character (cast `/Game/Character/Player/BP_Action_Character` (`GameplayStatics.GetPlayerCharacter` 0)))
  (if (`/Game/Character/Player/BP_Action_Character.Get Parry` _asbp_action_character)
    (`KismetSystemLibrary.PrintString` "パリィ成功")))

(event `テストＨＰ`
  (if (`self.isTest`)
    ;[0 1 0.3419] ウィジェットの作成
    (bind _returnvalue (`|CreateWidget` "/Game/Character/Enemies/Enemy1/WBP_ZombieBar.WBP_ZombieBar_C" (`GameplayStatics.GetPlayerController` 0)))
    (bind _output_get (set `self.HP_BarUI` _returnvalue))
    (set `/Game/Character/Enemies/Enemy1/WBP_ZombieBar.pParentChar` self _output_get)
    (`UserWidget.AddToViewport` _returnvalue 0)
    (set `self.isTest` false)))

(event `FinishStan`
  ;[1 1 0] スタン解除処理
  (set `self.isStan` false)
  (set `self.StanValue` 1.0)
  (`CharacterMovementComponent.SetMovementMode` (`self.CharacterMovement`) "MOVE_Walking" 0))

(event `self.Tackle_Collision.OnComponentBeginOverlap`
  (params (OverlappedComponent :type "PrimitiveComponent Object Reference") (OtherActor :type "Actor Object Reference") (OtherComp :type "PrimitiveComponent Object Reference") (OtherBodyIndex :type Integer) (bFromSweep :type Boolean) (SweepResult :type "HitResult Structure (by ref)"))
  (`KismetSystemLibrary.PrintString` (`KismetSystemLibrary.GetDisplayName` OtherActor))
  (if (!= OtherComp self)
    (bind _asbp_action_character (cast `/Game/Character/Player/BP_Action_Character` OtherActor))
    (if (== (`Character.CapsuleComponent` _asbp_action_character) OtherComp)
      (set `self.isAttackable` false)
      (`self.FinishTackle`)
      (`self.T_Attack`))))

(event `Tackle`
  ;[1 1 1] タックル
  (if (`BlackboardComponent.GetValueAsBool` (`AIBlueprintHelperLibrary.GetBlackboard` self) "TackleIdleFlag")
    (`self.K2_SetActorRotation` (`KismetMathLibrary.RInterpTo` (`self.K2_GetActorRotation`) (`KismetMathLibrary.FindLookAtRotation` (`self.K2_GetActorLocation`) (`self.K2_GetActorLocation` (`GameplayStatics.GetPlayerCharacter` 0))) (`GameplayStatics.GetWorldDeltaSeconds`) 4.0))
    (elif (`BlackboardComponent.GetValueAsBool` (`AIBlueprintHelperLibrary.GetBlackboard` self) "TackleFlag")
      (`self.ForwardAttack`)
      (`KismetSystemLibrary.Delay` 1.5)
      (`self.FinishTackle`)
      (if (`self.isAttackable`)
        (`self.T_Attack`)))))

(event `スタン処理`
  ;[1 1 0] スタン時の処理
  (set `self.isStan` true)
  (`self.OffAttackFlag`)
  (`MovementComponent.StopMovementImmediately` (`self.CharacterMovement`))
  (`self.SpawnStunEffect`)
  (`KismetSystemLibrary.PrintString` "スタン開始"))

(event `T_Attack`
  (`BlackboardComponent.SetValueAsBool` (`AIBlueprintHelperLibrary.GetBlackboard` self) "AttackFlag" true)
  (`KismetSystemLibrary.Delay` 2.81)
  (`BlackboardComponent.SetValueAsBool` (`AIBlueprintHelperLibrary.GetBlackboard` self) "AttackFlag" false)
  (`KismetSystemLibrary.Delay` 0.8)
  (`KismetSystemLibrary.PrintString` "ゾンビ）攻撃終了" true true (struct :`G` 0.058898 :`B` 1.0 :`A` 1.0))
  (set `self.isTacklable` true))

(event `self.ReceiveAnyDamage`
  (params (Damage :type "Float (single-precision)") (DamageType :type "DamageType Object Reference") (InstigatedBy :type "Controller Object Reference") (DamageCauser :type "Actor Object Reference"))
  ;[1 0.007369 0] プレイヤーからダメージを受けた時の処理
  ;;[0 0.8963 1] スタン中か否かの処理
  (if (not (`self.isStan`))
    (`self.Back`) ; プレイヤーが背後から攻撃したかの判定
    (`self.SetStanValue` 0.2)
    (`self.CheckIsStan`))
  (`self.SetHP` Damage)
  (bind _returnvalue (`NiagaraFunctionLibrary.SpawnSystemAtLocation` "/Game/Effect/EHit_Set/EHit.EHit" (`self.K2_GetActorLocation`) (struct) (0.25 0.25 0.25) true true "AutoRelease")) ; ダメージエフェクト
  (`KismetArrayLibrary.Array_Add` (`self.particles`) _returnvalue)
  (if (`self.isInvincible`)
    (set `self.isInvincible` false)
    (set `self.DamageCount` 0)
    (elif (`self.isBackDamaging`)
      (`self.SetBackDamage`)
      (else
        (`self.SetDamage`))))
  (`self.GetIsAlive`))

(event `self.Attack_Collision.OnComponentBeginOverlap`
  (params (OverlappedComponent :type "PrimitiveComponent Object Reference") (OtherActor :type "Actor Object Reference") (OtherComp :type "PrimitiveComponent Object Reference") (OtherBodyIndex :type Integer) (bFromSweep :type Boolean) (SweepResult :type "HitResult Structure (by ref)"))
  ;[1 0 0] プレイヤーにダメージを与える
  (if (not (`self.isStan`))
    (bind _asbp_action_character (cast `/Game/Character/Player/BP_Action_Character` OtherActor))
    (if (== (`Character.CapsuleComponent` _asbp_action_character) OtherComp)
      (`GameplayStatics.ApplyDamage` OtherActor 0.2 null self))))

(event `LookAtPlayer`
  ;[0 0.7559 1] プレイヤーの方向を向く
  (`self.K2_SetActorRotation` (`KismetMathLibrary.RInterpTo` (`self.K2_GetActorRotation`) (`KismetMathLibrary.FindLookAtRotation` (`self.K2_GetActorLocation`) (`self.K2_GetActorLocation` (`GameplayStatics.GetPlayerCharacter` 0))) (`GameplayStatics.GetWorldDeltaSeconds`) 4.0)))

(event `Back`
  (bind (_returnvalue_x _returnvalue_y) (`KismetMathLibrary.BreakVector` (`self.K2_GetActorLocation`)))
  (bind (_returnvalue_x_2 _returnvalue_y_2) (`KismetMathLibrary.BreakVector` (`self.K2_GetActorLocation` (`GameplayStatics.GetPlayerCharacter` 0))))
  (bind (_returnvalue_roll _returnvalue_pitch _returnvalue_yaw) (`KismetMathLibrary.BreakRotator` (`KismetMathLibrary.NormalizedDeltaRotator` (`self.K2_GetActorRotation`) (`self.K2_GetActorRotation` (`GameplayStatics.GetPlayerCharacter` 0)))))
  (bind _returnvalue (`KismetMathLibrary.Abs` _returnvalue_yaw))
  ;[1 0 0] プレイヤーが後ろから攻撃してきたら
  (`KismetSystemLibrary.PrintString` (`KismetStringLibrary.Concat_StrStr` "角度は：" (`KismetStringLibrary.Conv_DoubleToString` _returnvalue)) true true (struct :`R` 1.0 :`B` 0.115187 :`A` 1.0) 5.0)
  (bind _output_get (set `self.Degree` (`KismetMathLibrary.FTrunc` (`KismetMathLibrary.DegAtan2` (- (`KismetMathLibrary.MultiplyMultiply_FloatFloat` _returnvalue_y_2 2.0) (`KismetMathLibrary.MultiplyMultiply_FloatFloat` _returnvalue_y 2.0)) (- (`KismetMathLibrary.MultiplyMultiply_FloatFloat` _returnvalue_x_2 2.0) (`KismetMathLibrary.MultiplyMultiply_FloatFloat` _returnvalue_x 2.0))))))
  (if (<= _returnvalue 75.0)
    (set `self.isBack` true)
    (`KismetSystemLibrary.PrintString` "プレイヤーが後ろにいた" true true (struct :`R` 1.0 :`B` 0.131112 :`A` 1.0))
    (set `self.isBackDamaging` true)))

(event `SettingUI`
  (bind _hp_barui (`self.HP_BarUI`))
  ;[0 0.9131 1] ゲージの表示
  (if (`KismetSystemLibrary.IsValid` _hp_barui)
    (`/Game/Character/Enemies/Enemy1/WBP_ZombieBar.SetUpdateGaugePosition` _hp_barui self)))

(event `test`
  (bind (_returnvalue_roll _returnvalue_pitch _returnvalue_yaw) (`KismetMathLibrary.BreakRotator` (`KismetMathLibrary.NormalizedDeltaRotator` (`self.K2_GetActorRotation`) (`self.K2_GetActorRotation` (`GameplayStatics.GetPlayerCharacter` 0)))))
  ;[1 0 0] プレイヤーが後ろから攻撃してきたら
  (`KismetSystemLibrary.PrintString` (`KismetStringLibrary.Concat_StrStr` "角度は：" (`KismetStringLibrary.Conv_DoubleToString` (`KismetMathLibrary.Abs` _returnvalue_yaw))) true true (struct :`G` 1.0 :`B` 0.180375 :`A` 1.0) 0.5))

(event `Damage`
  ;[0 0.9131 1] ダメージ食らった時の処理
  (`KismetSystemLibrary.Delay` 1.0)
  (`self.FinishDamage`))

(event `BackDamage`
  ;[0 0.9131 1] ダメージ食らった時の処理
  (if (`self.isBackDamaging`)
    (`KismetSystemLibrary.Delay` 1.085)
    (`self.FinishBackDamage`)))

(fn `All Collision Off`
  (`PrimitiveComponent.SetCollisionEnabled` (`self.Attack_Collision`) "NoCollision")
  (`PrimitiveComponent.SetCollisionEnabled` (`self.CapsuleComponent`) "NoCollision"))

(fn `CheckIsStan`
  (bind _output_get (set `self.isStan` (<= (`self.StanValue`) 0.03)))
  (if _output_get
    (`KismetSystemLibrary.PrintString` "スタン値が溜まり切ったのでスタン状態になります" true true (struct :`R` 1.0 :`G` 0.845567 :`A` 1.0) 4.0)
    (`self.OffDamageFlag`)
    (`self.スタン処理`)))

(fn `Disappear Particle`
  (for _ (`self.particles`)
    _)
  (`KismetSystemLibrary.PrintString` "完了！！！"))

(fn `FinishBackDamage`
  (`BlackboardComponent.SetValueAsBool` (`AIBlueprintHelperLibrary.GetBlackboard` self) "BackDamageFlag" false)
  (set `self.isBackDamaging` false)
  (`self.CheckIsStan`)
  (`KismetSystemLibrary.PrintString` "背面からの攻撃処理終了")
  (`BlackboardComponent.SetValueAsBool` (`AIBlueprintHelperLibrary.GetBlackboard` self) "AttackFlag" true))

(fn `FinishDamage`
  (`BlackboardComponent.SetValueAsBool` (`AIBlueprintHelperLibrary.GetBlackboard` self) "DamageFlag" false)
  (set `self.isDamaging` false)
  (`self.CheckIsStan`)
  (`self.Notify DisActivate Attack Time`))

(fn `FinishTackle`
  (bind _returnvalue (`AIBlueprintHelperLibrary.GetBlackboard` self))
  (`BlackboardComponent.SetValueAsBool` _returnvalue "TackleHitFlag" true)
  (`BlackboardComponent.SetValueAsBool` _returnvalue "TackleFlag" false)
  (`PrimitiveComponent.SetCollisionEnabled` (`self.Tackle_Collision`) "NoCollision") ; 攻撃用の当たり判定をとれないようにする
)

(fn `ForwardAttack`
  (`self.K2_SetActorLocation` (+ (* (`KismetMathLibrary.GetForwardVector` (`self.K2_GetActorRotation`)) (* (`GameplayStatics.GetWorldDeltaSeconds`) (`self.TackleSpeed`))) (`self.K2_GetActorLocation`)) true))

(fn `GetAttackTime`
  (returns (isAttackTime :type Boolean))
  (return (`self.isAttackTime`)))

(fn `GetIsAlive`
  (bind _output_get (set `self.isDeath` (>= (`self.HP`) (`self.Max_HP`))))
  (if _output_get
    (set `/Game/Character/Enemies/Enemy1/WBP_ZombieBar.pParentChar` null (`self.HP_BarUI`))
    (`self.All Collision Off`)
    (`BlackboardComponent.SetValueAsBool` (`AIBlueprintHelperLibrary.GetBlackboard` self) "DeathFlag" true)
    (`self.Disappear Particle`)
    (if (`self.isDamaging`)
      (`self.FinishDamage`))))

(fn `GetIsStan`
  (returns (IsStan :type Boolean))
  (return (`self.isStan`)))

(fn `GetRandomLocation`
  (returns (Location :type "Vector Structure"))
  (bind _movearea (`self.MoveArea`))
  (bind (_origin _boxextent) (`KismetSystemLibrary.GetComponentBounds` (`TriggerBase.CollisionComponent` _movearea)))
  (`/Engine/EditorBlueprintResources/StandardMacros.IsValid` _movearea
    (:`Is Valid`
      (return (`KismetMathLibrary.RandomPointInBoundingBox` _origin _boxextent)))
    (:`Is Not Valid`
      (return (0.0 0.0 0.0)))))

(fn `Notify Activate Attack Time`
  (set `self.isAttackTime` true)
  (`PrimitiveComponent.SetCollisionEnabled` (`self.Attack_Collision`) "QueryAndPhysics"))

(fn `Notify DisActivate Attack Time`
  (set `self.isAttackTime` false)
  (`PrimitiveComponent.SetCollisionEnabled` (`self.Attack_Collision`) "NoCollision"))

(fn `OffAttackFlag`
  (bind _returnvalue (`AIBlueprintHelperLibrary.GetBlackboard` self))
  (`self.Notify DisActivate Attack Time`)
  (if (`BlackboardComponent.GetValueAsBool` _returnvalue "AttackFlag")
    (`BlackboardComponent.SetValueAsBool` _returnvalue "AttackFlag" false)))

(fn `OffDamageFlag`
  (set `self.isDamaging` false)
  (set `self.isBackDamaging` false)
  (`BlackboardComponent.SetValueAsBool` (`AIBlueprintHelperLibrary.GetBlackboard` self) "DamageFlag" false)
  (`BlackboardComponent.SetValueAsBool` (`AIBlueprintHelperLibrary.GetBlackboard` self) "BackDamageFlag" false))

(fn `SetAIContoller`
  (set `self.AIControllerClass` "/Game/Character/Enemies/Enemy1/AIC_Enemy1.AIC_Enemy1_C")
  (`AIController.RunBehaviorTree` (`AIBlueprintHelperLibrary.GetAIController` self) "/Game/Character/Enemies/Enemy1/BT_Enemy1.BT_Enemy1"))

(fn `SetBackDamage`
  (`BlackboardComponent.SetValueAsBool` (`AIBlueprintHelperLibrary.GetBlackboard` self) "BackDamageFlag" true))

(fn `SetBeginHp`
  (bind _returnvalue (`GameplayStatics.GetActorOfClass` "/Game/GameManager/EnemySpawnerManager.EnemySpawnerManager_C"))
  (set `self.Max_HP` (`/Game/GameManager/EnemySpawnerManager.EnemyHP` _returnvalue))
  ;[0 1 0.3419] ウィジェットの作成
  (bind _returnvalue_2 (`|CreateWidget` "/Game/Character/Enemies/Enemy1/WBP_ZombieBar.WBP_ZombieBar_C" (`GameplayStatics.GetPlayerController` 0)))
  (bind _output_get (set `self.HP_BarUI` _returnvalue_2))
  (set `/Game/Character/Enemies/Enemy1/WBP_ZombieBar.pParentChar` self _output_get)
  (`UserWidget.AddToViewport` _returnvalue_2 0))

(fn `SetDamage`
  (set `self.isDamaging` true)
  (`BlackboardComponent.SetValueAsBool` (`AIBlueprintHelperLibrary.GetBlackboard` self) "DamageFlag" true)
  (bind _result (`/Engine/EditorBlueprintResources/StandardMacros.IncrementInt` (`self.DamageCount`))
    (:`  `
      (if (>= _result 2)
        (set `self.isInvincible` true)))))

(fn `setEnemyColor`
  (if (`self.isTest`)
    (bind _returnvalue (`GameplayStatics.GetActorOfClass` "/Game/Character/Enemies/TestEnemyManager.TestEnemyManager_C"))
    (`MaterialInstanceDynamic.SetVectorParameterValue` (`self.MaterialInstance`) "BaseColor" (`KismetMathLibrary.Conv_ColorToLinearColor` (`|GetArrayItem` (`self.ColorTable`) (`/Game/Character/Enemies/TestEnemyManager.A_NUM` _returnvalue))))
    (else
      (bind _returnvalue_2 (`GameplayStatics.GetActorOfClass` "/Game/GameManager/EnemySpawnerManager.EnemySpawnerManager_C"))
      (`MaterialInstanceDynamic.SetVectorParameterValue` (`self.MaterialInstance`) "BaseColor" (`KismetMathLibrary.Conv_ColorToLinearColor` (`|GetArrayItem` (`self.ColorTable`) (`/Game/GameManager/EnemySpawnerManager.EnemiesMoveType` _returnvalue_2)))))))

(fn `SetHP`
  (params (Damage :type "Float (double-precision)"))
  (set `self.HP` (+ (`self.HP`) Damage)))

(fn `SetStanValue`
  (params (StanValue :type "Float (double-precision)"))
  (set `self.StanValue` (- (`self.StanValue`) StanValue)) ; スタン状態でなかったらスタン値をためる
)

(fn `SetStatus`)

(fn `SpawnStunEffect`)

(fn `StartTackle`
  (`PrimitiveComponent.SetCollisionEnabled` (`self.Tackle_Collision`) "QueryOnly") ; 攻撃用の当たり判定をとれないようにする
)

(fn `TackleAttack`
  (`BlackboardComponent.SetValueAsBool` (`AIBlueprintHelperLibrary.GetBlackboard` self) "AttackFlag" true))

(fn `UserConstructionScript`
  (bind _returnvalue (`PrimitiveComponent.CreateDynamicMaterialInstance` (`self.Mesh`) 0 "/Game/Resources/Textures/ZombieTextures/DefaultMaterial_Base_Color2_Mat.DefaultMaterial_Base_Color2_Mat" "None"))
  (set `self.MaterialInstance` _returnvalue))