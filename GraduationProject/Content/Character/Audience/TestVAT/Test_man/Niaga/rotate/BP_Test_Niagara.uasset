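; Test audience actor that switches a Niagara VAT (by its naming) crowd from group animation to individual animation.
; Tick polls IsPlayAllAnimAudience on TestGameInst, then briefly pulses User.IsPlayAll and passes PlayAllFrame as the start frame.
; After WaitSec it pulses User.IsPlaySingle and clears the game instance flag, with Delay nodes inside Tick sequencing the steps and debug prints marking start and reset.
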(event `self.ReceiveBeginPlay`)

(event `self.ReceiveTick`
  (params (DeltaSeconds :type "Float (single-precision)"))
  (bind _ns_vat (`self.NS_VAT`))
  (bind _ns_vat_2 (`self.NS_VAT`))
  ;[1 1 1] isPlayAll検知用 trueなら通る
  (bind _astest_game_inst (cast `/Game/Character/Audience/TestVAT/Test_man/TestGameInst` (`GameplayStatics.GetGameInstance`)))
  (if (`/Game/Character/Audience/TestVAT/Test_man/TestGameInst.IsPlayAllAnimAudience` _astest_game_inst)
    (`KismetSystemLibrary.PrintString` "集団アニメーション開始")
    (`KismetSystemLibrary.Delay` 0.01)
    ;[1 1 1] 集団アニメーション
    (`NiagaraComponent.SetVariableBool` _ns_vat "User.IsPlayAll" true)
    (`NiagaraComponent.SetVariableFloat` _ns_vat "User.PlayAllStatFrame" (`self.PlayAllFrame`))
    (`KismetSystemLibrary.Delay` 0.01)
    (`NiagaraComponent.SetVariableBool` _ns_vat "User.IsPlayAll" false)
    ;[1 1 1] 個別アニメーション
    (`KismetSystemLibrary.Delay` (`self.waitSec`))
    (`NiagaraComponent.SetVariableBool` _ns_vat_2 "User.IsPlaySingle" true)
    (`KismetSystemLibrary.Delay` 0.01)
    (`NiagaraComponent.SetVariableBool` _ns_vat_2 "User.IsPlaySingle" false)
    ;[1 1 1] falseへ
    (bind _astest_game_inst_2 (cast `/Game/Character/Audience/TestVAT/Test_man/TestGameInst` (`GameplayStatics.GetGameInstance`)))
    (set `/Game/Character/Audience/TestVAT/Test_man/TestGameInst.IsPlayAllAnimAudience` false _astest_game_inst_2)
    (`KismetSystemLibrary.PrintString` "flaseへ")))

(fn `UserConstructionScript`)