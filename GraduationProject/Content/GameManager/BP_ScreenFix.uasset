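; Actor Blueprint that forces the game's display mode and resolution through Game User Settings.
; The Construction Script applies Windowed mode at a fixed 1080p resolution.
; BeginPlay then switches to Windowed Fullscreen at the same resolution and applies it again, with command-line override checks enabled in both passes.
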(event `self.ReceiveBeginPlay`
  (bind _returnvalue (`GameUserSettings.GetGameUserSettings`))
  (`GameUserSettings.SetFullscreenMode` _returnvalue "WindowedFullscreen")
  (`GameUserSettings.SetScreenResolution` _returnvalue (make `IntPoint` 1920 1080))
  (`GameUserSettings.ApplySettings` _returnvalue true))

(fn `UserConstructionScript`
  (bind _returnvalue (`GameUserSettings.GetGameUserSettings`))
  (`GameUserSettings.SetFullscreenMode` _returnvalue "Windowed")
  (`GameUserSettings.SetScreenResolution` _returnvalue (make `IntPoint` 1920 1080))
  (`GameUserSettings.ApplySettings` _returnvalue true))